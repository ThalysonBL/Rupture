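; Base AI controller for Rupture enemies that tracks the player through AI perception.
; On possession it runs the behavior tree assigned on the enemy pawn itself, so each enemy supplies its own logic.
; Perception updates set TargetActor on the blackboard when the player is sensed.
; When the player is lost, it stores their current position as LastKnownLocation and clears TargetActor.
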(event `self.ReceivePossess`
  (params (PossessedPawn :type "Pawn Object Reference"))
  (bind _asrupture_enemy_base (cast `RuptureEnemyBase` PossessedPawn))
  (`self.RunBehaviorTree` (`RuptureEnemyBase.EnemyBehaviorTree` _asrupture_enemy_base)))

(event `self.AIPerception.OnTargetPerceptionUpdated`
  (params (Actor :type "Actor Object Reference") (Stimulus :type "AIStimulus Structure"))
  (bind _returnvalue (`AIBlueprintHelperLibrary.GetBlackboard` null))
  (bind _asbp_rupture_player_character (cast `/Game/Blueprints/Characters/BP_RupturePlayerCharacter` Actor))
  (if (`.bSuccessfullySensed` (break `AIStimulus` Stimulus))
    ; Encontra o player
    (`BlackboardComponent.SetValueAsObject` (`AIBlueprintHelperLibrary.GetBlackboard` null) "TargetActor" _asbp_rupture_player_character)
    (`BlackboardComponent.ClearValue` (`AIBlueprintHelperLibrary.GetBlackboard` null) "LastKnownLocation")
    (else
      ; lost sight of the character
      (`BlackboardComponent.SetValueAsVector` _returnvalue "LastKnownLocation" (`self.K2_GetActorLocation` _asbp_rupture_player_character))
      (`BlackboardComponent.ClearValue` _returnvalue "TargetActor"))))

(fn `UserConstructionScript`)