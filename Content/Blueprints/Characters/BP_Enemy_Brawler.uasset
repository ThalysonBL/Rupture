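; BP_Enemy_Brawler is a melee enemy that damages the Rupture player character through left and right sphere hitboxes.
; AttackMeleeEvent plays the attack montage, while separate events enable and disable query collision on both spheres to open and close the damage window.
; Both overlaps share one DoOnce, reset when damage is disabled, so the player takes a fixed hit only once per window.
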(event `self.Sphere_Right.OnComponentBeginOverlap`
  (params (OverlappedComponent :type "PrimitiveComponent Object Reference") (OtherActor :type "Actor Object Reference") (OtherComp :type "PrimitiveComponent Object Reference") (OtherBodyIndex :type Integer) (bFromSweep :type Boolean) (SweepResult :type "HitResult Structure (by ref)"))
  ; Apply Damage
  (bind _asbp_rupture_player_character (cast `/Game/Blueprints/Characters/BP_RupturePlayerCharacter` (stale `self.Sphere_Left.OnComponentBeginOverlap` OtherActor) :!label _label))
  (`/Engine/EditorBlueprintResources/StandardMacros.DoOnce` false :!label _label_2
    (:`Completed`
      (`GameplayStatics.ApplyDamage` _asbp_rupture_player_character 20.0 null self))))

(event `self.Sphere_Left.OnComponentBeginOverlap`
  (params (OverlappedComponent :type "PrimitiveComponent Object Reference") (OtherActor :type "Actor Object Reference") (OtherComp :type "PrimitiveComponent Object Reference") (OtherBodyIndex :type Integer) (bFromSweep :type Boolean) (SweepResult :type "HitResult Structure (by ref)"))
  ; Apply Damage
  (goto _label))

(event `ActiveDamageEvent`
  ; Apply Damage
  (`PrimitiveComponent.SetCollisionEnabled` (`self.Sphere_Left`) "QueryOnly")
  (`PrimitiveComponent.SetCollisionEnabled` (`self.Sphere_Right`) "QueryOnly"))

(event `DisableDamageEvent`
  ; Apply Damage
  (`PrimitiveComponent.SetCollisionEnabled` (`self.Sphere_Left`) "NoCollision")
  (`PrimitiveComponent.SetCollisionEnabled` (`self.Sphere_Right`) "NoCollision")
  (goto _label_2 :!via `Reset`))

(event `AttackMeleeEvent`
  ; Attack Anim Montage
  (`|PlayMontage` (`self.Mesh`) "/Game/FreeAnimationLibrary/Animations/Counter-Finisher/AM_CounterAttack_using.AM_CounterAttack_using"))

(fn `UserConstructionScript`)